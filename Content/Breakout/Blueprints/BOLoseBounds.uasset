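; BOLoseBounds is the lose boundary for the Breakout game, pausing play and showing reset text when it is hit.
; BeginPlay finds the BO_PauseText actor with GetActorOfClass and caches its transform.
; The Hit event pauses the game and spawns BO_ResetText at that transform, without filtering what hit it.
; An older GetAllActorsOfClass lookup remains disconnected and never runs.
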(event `self.ReceiveBeginPlay`
  ;[1 1 1] Optimized, doesn't have to iterate through classes, just finds the one class.
  (bind _returnvalue (`GameplayStatics.GetActorOfClass` "/Game/Breakout/Blueprints/BO_PauseText.BO_PauseText_C"))
  (set `self.TextTransform` (`self.GetTransform` _returnvalue)))

(event `self.ReceiveHit`
  (params (MyComp :type "PrimitiveComponent Object Reference") (Other :type "Actor Object Reference") (OtherComp :type "PrimitiveComponent Object Reference") (bSelfMoved :type Boolean) (HitLocation :type "Vector Structure") (HitNormal :type "Vector Structure") (NormalImpulse :type "Vector Structure") (Hit :type "HitResult Structure (by ref)"))
  (`GameplayStatics.SetGamePaused` true)
  (`|SpawnActorFromClass` "/Game/Breakout/Blueprints/BO_ResetText.BO_ResetText_C" (`self.TextTransform`) "Undefined" "OverrideRootScale" null null))

(fn `UserConstructionScript`)