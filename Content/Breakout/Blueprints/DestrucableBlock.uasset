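; Destructible brick actor for a Breakout game that destroys itself when hit.
; The Construction Script creates a dynamic material instance on the block mesh.
; On BeginPlay that material's BlockColor is set to a random green-dominant tint, with full green and varied red and blue.
; A Hit event waits a very brief delay before destroying the actor.
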(event `self.ReceiveBeginPlay`
  (`MaterialInstanceDynamic.SetVectorParameterValue` (`self.BlockMeshMat`) "BlockColor" (make `LinearColor` (`KismetMathLibrary.RandomFloatInRange` 0.0 0.75) (`KismetMathLibrary.RandomFloatInRange` 1.0 1.0) (`KismetMathLibrary.RandomFloatInRange` 0.0 0.75) 1.0)))

(event `self.ReceiveHit`
  (params (MyComp :type "PrimitiveComponent Object Reference") (Other :type "Actor Object Reference") (OtherComp :type "PrimitiveComponent Object Reference") (bSelfMoved :type Boolean) (HitLocation :type "Vector Structure") (HitNormal :type "Vector Structure") (NormalImpulse :type "Vector Structure") (Hit :type "HitResult Structure (by ref)"))
  (`KismetSystemLibrary.Delay` 0.01)
  (`self.K2_DestroyActor`))

(fn `UserConstructionScript`
  (bind _returnvalue (`PrimitiveComponent.CreateDynamicMaterialInstance` (`self.BlockMesh`) 0 "/Game/Breakout/Materials/BOBlockMat.BOBlockMat" "None"))
  (set `self.BlockMeshMat` _returnvalue))